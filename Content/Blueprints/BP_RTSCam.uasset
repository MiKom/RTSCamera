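; RTS camera pawn or actor that pans along its yaw and zooms on a spring arm.
; Zoom events step a clamped target length by a curve-scaled rate based on current arm length, which Tick interpolates toward.
; Tick also sums movement and edge axes, set outside these graphs, into a clamped, swept move without delta-time scaling.
; The construction script's camera setup is disconnected.
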(event Custom|ZoomIn
  (bind _cameraboom (Variables|Default|GetCameraBoom))
  (bind _targetarmlength (Variables|/Script/Engine.SpringArmComponent|GetTargetArmLength _cameraboom))
  ;[1 1 1] Zoom Events
  (Variables|CommandCam|SetCameraBoomLength (Math|Float|Clamp(Float) (- _targetarmlength (* (Math|Curves|GetFloatValue (Variables|CommandCam|GetZoomRateCurve) _targetarmlength) (Variables|CommandCam|GetBaseZoomRate))) (Variables|CommandCam|GetMinZoom) (Variables|CommandCam|GetMaxZoom))))

(event Custom|ZoomOut
  (bind _cameraboom (Variables|Default|GetCameraBoom))
  (bind _targetarmlength (Variables|/Script/Engine.SpringArmComponent|GetTargetArmLength _cameraboom))
  ;[1 1 1] Zoom Events
  (Variables|CommandCam|SetCameraBoomLength (Math|Float|Clamp(Float) (+ _targetarmlength (* (Math|Curves|GetFloatValue (Variables|CommandCam|GetZoomRateCurve) _targetarmlength) (Variables|CommandCam|GetBaseZoomRate))) (Variables|CommandCam|GetMinZoom) (Variables|CommandCam|GetMaxZoom))))

(event EventTick
  (params (DeltaSeconds :type Float%20%28single-precision%29))
  (bind _returnvalue (Utilities|IsolateYaw))
  (bind _cameraboom (Variables|Default|GetCameraBoom))
  ;[1 1 1] Zoom Interp
  (Variables|/Script/Engine.SpringArmComponent|SetTargetArmLength _cameraboom (Math|Interpolation|FInterpTo (Variables|/Script/Engine.SpringArmComponent|GetTargetArmLength _cameraboom) (Variables|CommandCam|GetCameraBoomLength) DeltaSeconds (Variables|CommandCam|GetCameraZoomSpeed)))
  ;[1 1 1] Camera WASD Movement
  (Variables|Default|SetCameraPan (+ (+ (* (Math|Vector|GetForwardVector _returnvalue) (Math|Float|Clamp(Float) (+ (Variables|Default|GetMoveForwardAxis) (Variables|CommandCam|GetEdgeForwardAxis)) -1e+01 1e+01)) (* (Math|Vector|GetRightVector _returnvalue) (Math|Float|Clamp(Float) (+ (Variables|Default|GetMoveLateralAxis) (Variables|CommandCam|GetEdgeLateralAxis)) -1e+01 1e+01))) (Transformation|GetWorldLocation)))
  (Transformation|SetActorLocation (Variables|Default|GetCameraPan) true))

(fn ConstructionScript)