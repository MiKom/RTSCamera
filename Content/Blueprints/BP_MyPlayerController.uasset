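; BP_MyPlayerController is the player controller that forwards camera input to the BP_RTSCam pawn for an RTS-style view.
; Move axes write the pawn's forward and lateral movement values, and zoom actions call its zoom in and out functions.
; Holding middle mouse lets the rotation axis yaw the camera boom by the pawn's rotation speed, with pitch held fixed.
; Each input event casts player pawn 0 to BP_RTSCam itself.
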(event Input|ActionEvents|InputActionCameraZoomIn
  ;[1 1 1] Camera Zoom (Communicates with RTS Cam)
  (:Pressed
    (bind _asbp_rtscam (Utilities|Casting|CastToBP_RTSCam (Game|Player|GetPlayerPawn 0)))
    (Default|Zoomin _asbp_rtscam)))

(event Input|ActionEvents|InputActionCameraZoomOut
  ;[1 1 1] Camera Zoom (Communicates with RTS Cam)
  (:Pressed
    (bind _asbp_rtscam (Utilities|Casting|CastToBP_RTSCam (Game|Player|GetPlayerPawn 0)))
    (Default|ZoomOut _asbp_rtscam)))

(event Input|AxisEvents|InputAxisCameraRotation
  (params (AxisValue :type Float%20%28single-precision%29))
  ;[1 1 1] Camera Rotation [Communicates with RTS Cam]
  (bind _asbp_rtscam (Utilities|Casting|CastToBP_RTSCam (Game|Player|GetPlayerPawn 0)))
  (if (Game|Player|IsInputKeyDown "MiddleMouseButton")
    (Transformation|SetRelativeRotation (Variables|/Game/Blueprints/BP_RTSCam.BP_RTSCam_C|GetCameraBoom _asbp_rtscam) (Class|KismetMathLibrary|MakeRot -6e+01 (+ (.Yaw (Class|KismetMathLibrary|BreakRot (Variables|/Script/Engine.SceneComponent|GetRelativeRotation (Variables|/Game/Blueprints/BP_RTSCam.BP_RTSCam_C|GetCameraBoom _asbp_rtscam)))) (* AxisValue (Variables|/Game/Blueprints/BP_RTSCam.BP_RTSCam_C|GetCameraRotationSpeed _asbp_rtscam))) 0.0) false)))

(event Input|AxisEvents|InputAxisMoveForward
  (params (AxisValue :type Float%20%28single-precision%29))
  ;[1 1 1] Camera Movement [Communicates with Cam]
  (bind _asbp_rtscam (Utilities|Casting|CastToBP_RTSCam (Game|Player|GetPlayerPawn 0)))
  (Variables|/Game/Blueprints/BP_RTSCam.BP_RTSCam_C|SetMoveForwardAxis _asbp_rtscam AxisValue))

(event Input|AxisEvents|InputAxisMoveRight
  (params (AxisValue :type Float%20%28single-precision%29))
  ;[1 1 1] Camera Movement [Communicates with Cam]
  (bind _asbp_rtscam (Utilities|Casting|CastToBP_RTSCam (Game|Player|GetPlayerPawn 0)))
  (Variables|/Game/Blueprints/BP_RTSCam.BP_RTSCam_C|SetMoveLateralAxis _asbp_rtscam AxisValue))

(fn ConstructionScript)